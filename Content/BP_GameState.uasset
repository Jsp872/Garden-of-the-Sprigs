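; Game state Blueprint that keeps the game's resource stock as an array of typed amounts.
; AddResource and RemoveResource adjust the amount of each entry matching a type, write it back, then call RefreshResources on the Test reference.
; HasEnoughResources checks a cost list against the stock by nested loops, failing on any matching type that falls short.
; RemoveResource does no sufficiency check itself, and BeginPlay and Tick are empty.
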(event EventBeginPlay)

(event EventTick
  (params (DeltaSeconds :type Float%20%28single-precision%29)))

(fn ConstructionScript)

(fn AddResource
  (params (ResourceType :type E_ResourceType%20Enum :default "NewEnumerator0") (AmountToAdd :type Integer))
  (for (_array_element _array_index) (Variables|Default|GetResources)
    (if (Utilities|Enum|Equal(Enum) (.Type (Utilities|Struct|BreakS_ResourceData _array_element)) ResourceType)
      (Utilities|Array|SetArrayElem (Variables|Default|GetResources) _array_index (Utilities|Struct|MakeS_ResourceData (.Type (Utilities|Struct|BreakS_ResourceData _array_element)) (+ (.Amount (Utilities|Struct|BreakS_ResourceData _array_element)) AmountToAdd)))
      (Default|RefreshResources (Variables|Default|Gettest)))))

(fn HasEnoughResources
  (params (Resources :type Array%20of%20S%20Resource%20Data%20Structures))
  (for _array_element Resources
    (for _array_element_2 (Variables|Default|GetResources)
      (if (Utilities|Enum|Equal(Enum) (.type _array_element) (.type _array_element_2))
        (if (not (>= (.amount _array_element_2) (.amount _array_element)))
          (return false)))))
  (return true))

(fn RemoveResource
  (params (ResourceType :type E_ResourceType%20Enum :default "NewEnumerator0") (AmountToRemove :type Integer))
  (for (_array_element _array_index) (Variables|Default|GetResources)
    (if (Utilities|Enum|Equal(Enum) (.Type (Utilities|Struct|BreakS_ResourceData _array_element)) ResourceType)
      (Utilities|Array|SetArrayElem (Variables|Default|GetResources) _array_index (Utilities|Struct|MakeS_ResourceData (.Type (Utilities|Struct|BreakS_ResourceData _array_element)) (- (.Amount (Utilities|Struct|BreakS_ResourceData _array_element)) AmountToRemove)))
      (Default|RefreshResources (Variables|Default|Gettest)))))