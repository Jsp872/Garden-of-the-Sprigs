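; BP_PassiveGameMode is a game mode that tracks the villager population and decides when the game is won or lost.
; On BeginPlay it caches the first BP_Campfire in the level.
; CheckGameState sends the AllVillagers count to the Minpik counter in the player controller's main UI.
; It then shows WBP_EndScreen as a defeat when no villagers remain, or flagged as a victory at one hundred or more.
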(event EventBeginPlay
  (bind _outactors (Actor|GetAllActorsOfClass "/Game/Blueprint/Building/BP_Campfire.BP_Campfire_C"))
  (Variables|Default|SetCampfireRef (Utilities|Array|Get(acopy) _outactors)))

(event EventTick
  (params (DeltaSeconds :type Float%20%28single-precision%29)))

(fn ConstructionScript)

(fn CheckGameState
  (bind _allvillagers (Variables|Default|GetAllVillagers))
  (bind _returnvalue (Utilities|Array|Length _allvillagers))
  (Default|UpdateMinpikCounter (Variables|/Game/Blueprint/Core/BP_PassivePlayerController.BP_PassivePlayerController_C|GetMainUi (.AsBP%20Passive%20Player%20Controller (Utilities|Casting|CastToBP_PassivePlayerController (Game|GetPlayerController 0)))) _returnvalue)
  (if (<= _returnvalue 0)
    (bind _returnvalue_2 (UserInterface|CreateWidget "/Game/Blueprint/UI/WBP_EndScreen.WBP_EndScreen_C"))
    (UserInterface|Viewport|AddtoViewport _returnvalue_2 0)
    (elif (>= _returnvalue 100)
      (bind _returnvalue_3 (UserInterface|CreateWidget "/Game/Blueprint/UI/WBP_EndScreen.WBP_EndScreen_C"))
      (Variables|/Game/Blueprint/UI/WBP_EndScreen.WBP_EndScreen_C|SetIsVictory _returnvalue_3 true)
      (UserInterface|Viewport|AddtoViewport _returnvalue_3 0))))