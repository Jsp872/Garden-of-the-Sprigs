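; BP_BuildingBase is the base Blueprint for placeable buildings, including their placement preview.
; While in preview, Tick tints the Cube mesh green or red depending on CanPlace.
; CanPlace requires the Sphere to overlap no actors and the game state to afford the cost of the player controller's selected building.
; A separate event disables the Cube's collision.
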(event Custom|DesactivateCollision
  (Collision|SetCollisionEnabled (Variables|Default|GetCube) "NoCollision"))

(event EventTick
  (params (DeltaSeconds :type Float%20%28single-precision%29))
  (bind _cube (Variables|Default|GetCube))
  (if (Variables|Default|GetIsPreview)
    (bind _can (CallFunction|CanPlace))
    (if _can
      (Rendering|Material|SetMaterial _cube 0 "/Game/Materials/M_Green.M_Green")
      (else
        (Rendering|Material|SetMaterial _cube 0 "/Game/Materials/M_Red.M_Red")))))

(fn ConstructionScript)

(fn CanPlace
  (if (<= (Utilities|Array|Length (Collision|GetOverlappingActors (Variables|Default|GetSphere) 0 :!class /Script/Engine.PrimitiveComponent)) 0)
    (bind _have (Default|HasEnoughResources (.AsBP%20Game%20State (Utilities|Casting|CastToBP_GameState (Game|GetGameState))) (.cost (Variables|/Game/Blueprint/Core/BP_PassivePlayerController.BP_PassivePlayerController_C|GetSelectedBuilding (.AsBP%20Passive%20Player%20Controller (Utilities|Casting|CastToBP_PassivePlayerController (Game|GetPlayerController 0)))))))
    (if _have
      (return true)
      (else
        (return false)))
    (else
      (return false))))