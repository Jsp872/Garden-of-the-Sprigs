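; Player controller for a cursor-driven builder game that handles building placement and villager selection.
; While placing, a preview follows the cursor trace; right click cancels, and left click spawns the selected building if placement and BP_GameState resources allow, then deducts its cost.
; Otherwise, left click toggles villager menus through CurrentMinpik.
; BeginPlay creates the main HUD, hands it to the game state, shows the cursor and adds Enhanced Input contexts.
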(event EventBeginPlay
  (bind _returnvalue (Game|GetPlayerController 0))
  (bind _returnvalue_2 (UserInterface|CreateWidget "/Game/Blueprint/UI/WBP_MainHUD.WBP_MainHUD_C"))
  (Variables|Default|SetMainUi _returnvalue_2)
  (UserInterface|Viewport|AddtoViewport _returnvalue_2 0)
  (Default|RefreshResources _returnvalue_2)
  (Variables|/Game/Blueprint/Core/BP_GameState.BP_GameState_C|Settest (.AsBP%20Game%20State (Utilities|Casting|CastToBP_GameState (Game|GetGameState))) _returnvalue_2)
  (Variables|/Script/Engine.PlayerController|SetbShowMouseCursor _returnvalue true)
  (Variables|/Script/Engine.PlayerController|SetbEnableClickEvents _returnvalue true)
  (if (Pawn|IsLocalPlayerController)
    (Utilities|FlowControl|Sequence
      (:then_0
        ;[1 1 1] Add regular input mappings
        (Input|AddMappingContext (PlayerController|LocalPlayerSubsystems|GetEnhancedInputLocalPlayerSubsystem) "/Game/Input/IMC_Combat.IMC_Combat" 0 "(bIgnoreAllPressedKeysUntilRelease=True,bForceImmediately=False,bNotifyUserSettings=False)")
        (Input|AddMappingContext (PlayerController|LocalPlayerSubsystems|GetEnhancedInputLocalPlayerSubsystem) "/Game/Input/IMC_MouseLook.IMC_MouseLook" 0 "(bIgnoreAllPressedKeysUntilRelease=True,bForceImmediately=False,bNotifyUserSettings=False)")))))

(event EventTick
  (params (DeltaSeconds :type Float%20%28single-precision%29))
  (if (Variables|Default|GetIsPlacingBuilding)
    (Transformation|SetActorLocation (Variables|Default|GetPreviewBuilding) (.Location (Collision|BreakHitResult (.HitResult (Game|Player|GetHitResultUnderCursorbyChannel "TraceTypeQuery1" true)))) false false)))

(event Input|MouseEvents|LeftMouseButton
  (params (Key :type Key%20Structure :default "None"))
  (bind _returnvalue (Game|GetGameState))
  (bind _selectedbuilding (Variables|Default|GetSelectedBuilding))
  (bind _asbp_game_state (Utilities|Casting|CastToBP_GameState _returnvalue))
  (:Pressed
    (if (Variables|Default|GetIsPlacingBuilding)
      (bind _can (Default|CanPlace (Variables|Default|GetPreviewBuilding)))
      (if _can
        (bind _have (Default|HasEnoughResources _asbp_game_state (.cost _selectedbuilding)))
        (if _have
          (Game|SpawnActorfromClass (.buildingclass _selectedbuilding) (Math|Conversions|ToTransform(Vector) (Transformation|GetActorLocation (Variables|Default|GetPreviewBuilding))) "Undefined" "MultiplyWithRoot" 0 false 0)
          (Actor|DestroyActor (Variables|Default|GetPreviewBuilding))
          (Variables|Default|SetIsPlacingBuilding false)
          (for _array_element (.cost _selectedbuilding)
            (Default|RemoveResource _asbp_game_state (.type _array_element) (.amount _array_element)))))
      (else
        (bind _asbp_villager (Utilities|Casting|CastToBP_Villager (.HitActor (Collision|BreakHitResult (.HitResult (Game|Player|GetHitResultUnderCursorbyChannel "TraceTypeQuery1" true)))))
          (:then
            (Utilities|IsValid (Variables|Default|GetCurrentMinpik)
              (:Is%20Valid
                (Default|HideMenu (Variables|Default|GetCurrentMinpik)))
              (:Is%20Not%20Valid
                _))
            (bind _output_get (Variables|Default|SetCurrentMinpik _asbp_villager))
            (Default|ShowMenu _output_get))
          (:CastFailed
            (Utilities|IsValid (Variables|Default|GetCurrentMinpik)
              (:Is%20Valid
                (Default|HideMenu (Variables|Default|GetCurrentMinpik))
                (Variables|Default|SetCurrentMinpik 0)))))))))

(event Input|MouseEvents|RightMouseButton
  (params (Key :type Key%20Structure :default "None"))
  (:Pressed
    (if (Variables|Default|GetIsPlacingBuilding)
      (Actor|DestroyActor (Variables|Default|GetPreviewBuilding))
      (Variables|Default|SetIsPlacingBuilding false))))

(fn ConstructionScript)