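; Minpik villager pawn that goes on timed resource expeditions and can pray to earn a resource periodically.
; Its state feeds an AI Blackboard, and a camera-facing widget serves as its menu.
; Type sets material and perks: Rouge boosts rewards, Blanc halves DeathChance.
; Expeditions hide it until a timer grants rewards; mismatched types risk destruction when a random roll exceeds DeathChance, triggering a GameMode state check.
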(event Custom|StartExpedition
  (params (CurrentExpedition :type S%20Expedition%20Structure) (MinpikBonus :type Integer))
  (Variables|Default|SetCurrentState "NewEnumerator2")
  (Rendering|SetActorHiddenInGame true)
  (Collision|SetActorEnableCollision false)
  (Utilities|Time|SetTimerbyEvent (delegate Custom|ReturnFromExpedition) (.duration CurrentExpedition)))

(event Custom|ReturnFromExpedition
  (bind _returnvalue (Game|GetGameState))
  (bind _asbp_game_state (Utilities|Casting|CastToBP_GameState _returnvalue))
  (CallFunction|CheckifMinpikSurvive (.recommendedtype (stale Custom|StartExpedition CurrentExpedition)))
  (Utilities|Time|ClearandInvalidateTimerbyHandle (Variables|Default|GetPrayEvent))
  (Rendering|SetActorHiddenInGame false)
  (Collision|SetActorEnableCollision true)
  (Variables|Default|SetCurrentState "NewEnumerator0")
  (for _array_element (.possiblerewards (stale Custom|StartExpedition CurrentExpedition))
    (if (Utilities|Enum|Equal(Enum) (Variables|Default|GetMinpikType) "NewEnumerator0")
      (Default|AddResource _asbp_game_state (.type (.resourcetype _array_element)) (* (+ (Math|Random|RandomIntegerinRange (.minamount _array_element) (.maxamount _array_element)) (* (.multiplier (stale Custom|StartExpedition CurrentExpedition)) (Math|Random|RandomIntegerinRange (.minamount _array_element) (.maxamount _array_element)))) 1.5))
      (else
        (Default|AddResource _asbp_game_state (.type (.resourcetype _array_element)) (+ (Math|Random|RandomIntegerinRange (.minamount _array_element) (.maxamount _array_element)) (* (.multiplier (stale Custom|StartExpedition CurrentExpedition)) (Math|Random|RandomIntegerinRange (.minamount _array_element) (.maxamount _array_element)))))))))

(event Custom|StartPray
  (bind _returnvalue (Utilities|Time|SetTimerbyEvent (delegate Custom|AddPray) 1e+01 true))
  (Variables|Default|SetPrayEvent _returnvalue))

(event Custom|AddPray
  (Default|AddResource (.AsBP%20Game%20State (Utilities|Casting|CastToBP_GameState (Game|GetGameState))) "NewEnumerator7" 1))

(event EventTick
  (params (DeltaSeconds :type Float%20%28single-precision%29))
  (Transformation|SetWorldRotation (Variables|Default|GetWidget) (Math|Rotator|FindLookatRotation (Transformation|GetWorldLocation (Variables|Default|GetWidget)) (Camera|GetCameraLocation (Game|GetPlayerCameraManager 0))) false false))

(event EventBeginPlay
  (Variables|/Game/Blueprint/UI/WBP_VillagerMenu.WBP_VillagerMenu_C|SetMinpikRef (.AsWBP%20Villager%20Menu (Utilities|Casting|CastToWBP_VillagerMenu (UserInterface|GetUserWidgetObject (Variables|Default|GetWidget)))) self)
  (bind _output_get (Variables|Default|SetBlackboard (Variables|/Script/AIModule.AIController|GetBlackboard (.AsBP%20AIController%20Minpik (Utilities|Casting|CastToBP_AIController_Minpik (Pawn|GetController))))))
  (AI|Components|Blackboard|SetValueasEnum _output_get (Variables|Default|GetKey%20Name) (Variables|Default|GetCurrentState))
  (bind _asbp_game_mode (Utilities|Casting|CastToBP_GameMode (Game|GetGameMode)))
  (Variables|Default|SetCampfireRef (Variables|/Game/Blueprint/Core/BP_GameMode.BP_GameMode_C|GetCampfireRef _asbp_game_mode))
  (Utilities|Array|Add (Variables|/Game/Blueprint/Core/BP_GameMode.BP_GameMode_C|GetAllMinpiks _asbp_game_mode) self)
  (switch Utilities|FlowControl|Switch|SwitchonE_MinpikType (Variables|Default|GetMinpikType)
    (:NewEnumerator0
      (for (_ _array_index) (Rendering|Material|GetMaterials (Variables|Character|GetMesh))
        (Rendering|Material|SetMaterial (Variables|Character|GetMesh) _array_index "/Game/Materials/M_Red.M_Red")))
    (:NewEnumerator1
      (Variables|Default|SetDeathChance (/ (Variables|Default|GetDeathChance) 2.0))
      (for (_ _array_index_2) (Rendering|Material|GetMaterials (Variables|Character|GetMesh))
        (Rendering|Material|SetMaterial (Variables|Character|GetMesh) _array_index_2 "/Game/Materials/M_White.M_White")))))

(fn ConstructionScript)

(fn ShowMenu
  (Rendering|SetVisibility (Variables|Default|GetWidget) true false))

(fn HideMenu
  (Rendering|SetVisibility (Variables|Default|GetWidget) false false))

(fn UpdateBlackboardState
  (params (NewState :type E_VillagerState%20Enum :default "NewEnumerator0"))
  (bind _output_get (Variables|Default|SetCurrentState NewState))
  (AI|Components|Blackboard|SetValueasEnum (Variables|Default|GetBlackboard) (Variables|Default|GetKey%20Name) _output_get)
  (CallFunction|HideMenu)
  (Variables|/Game/Blueprint/Core/BP_PlayerController.BP_PlayerController_C|SetCurrentMinpik (.AsBP%20Player%20Controller (Utilities|Casting|CastToBP_PlayerController (Game|GetPlayerController 0))) 0))

(fn CheckifMinpikSurvive
  (params (SafeType :type E_MinpikType%20Enum :default "NewEnumerator0"))
  (if (or (Utilities|Enum|Equal(Enum) SafeType "NewEnumerator2") (Utilities|Enum|Equal(Enum) SafeType (Variables|Default|GetMinpikType)))
    (return)
    (elif (>= (Variables|Default|GetDeathChance) (Math|Random|RandomFloatinRange 0.0 1.0))
      (return)
      (else
        (Utilities|Array|RemoveItem (Variables|/Game/Blueprint/Core/BP_GameMode.BP_GameMode_C|GetAllMinpiks (.AsBP%20Game%20Mode (Utilities|Casting|CastToBP_GameMode (Game|GetGameMode)))) self)
        (Default|CheckGameState (.AsBP%20Game%20Mode (Utilities|Casting|CastToBP_GameMode (Game|GetGameMode))))
        (Actor|DestroyActor)))))