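; BP_RedHouse is a placeable house Blueprint that adds a villager to the game when it begins play.
; Unless it is flagged as a preview, BeginPlay spawns a BP_Villager at the house's location, then has BP_PassiveGameMode check the game state.
; Its construction script only calls the parent's version.
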(event EventBeginPlay
  (if (not (Variables|Default|GetIsPreview))
    (Game|SpawnActorfromClass "/Game/BP_Villager.BP_Villager_C" (Math|Conversions|ToTransform(Vector) (Transformation|GetActorLocation self)) "Undefined" "MultiplyWithRoot" 0 "NewEnumerator0" 0)
    (Default|CheckGameState (.AsBP%20Passive%20Game%20Mode (Utilities|Casting|CastToBP_PassiveGameMode (Game|GetGameMode))))))

(fn ConstructionScript
  (|CallParentFunction))