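; Game mode that tracks the Minpik population and decides victory or defeat.
; On BeginPlay it caches a reference to the first campfire found in the level.
; CheckGameState pushes the AllMinpiks count to the player controller's main UI.
; It then shows the end screen as a defeat when none remain, or as a victory once there are at least a hundred.
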(event EventBeginPlay
  (bind _outactors (Actor|GetAllActorsOfClass "/Game/Blueprint/Building/BP_Campfire.BP_Campfire_C"))
  (Variables|Default|SetCampfireRef (Utilities|Array|Get(acopy) _outactors)))

(fn ConstructionScript)

(fn CheckGameState
  (bind _allminpiks (Variables|Default|GetAllMinpiks))
  (bind _returnvalue (Utilities|Array|Length _allminpiks))
  (Default|UpdateMinpikCounter (Variables|/Game/Blueprint/Core/BP_PlayerController.BP_PlayerController_C|GetMainUi (.AsBP%20Player%20Controller (Utilities|Casting|CastToBP_PlayerController (Game|GetPlayerController 0)))) _returnvalue)
  (if (<= _returnvalue 0)
    (bind _returnvalue_2 (UserInterface|CreateWidget "/Game/Blueprint/UI/WBP_EndScreen.WBP_EndScreen_C"))
    (UserInterface|Viewport|AddtoViewport _returnvalue_2 0)
    (elif (>= _returnvalue 100)
      (bind _returnvalue_3 (UserInterface|CreateWidget "/Game/Blueprint/UI/WBP_EndScreen.WBP_EndScreen_C"))
      (Variables|/Game/Blueprint/UI/WBP_EndScreen.WBP_EndScreen_C|SetIsVictory _returnvalue_3 true)
      (UserInterface|Viewport|AddtoViewport _returnvalue_3 0))))