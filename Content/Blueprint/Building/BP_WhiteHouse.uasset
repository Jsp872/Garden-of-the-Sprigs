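; White House building Blueprint that adds a Minpik to the game when it is placed as a real, non-preview building.
; On BeginPlay, if IsPreview is false, it spawns a BP_Minpik of a fixed type at its own location, then asks BP_GameMode to run CheckGameState.
; The construction script only calls its parent.
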(event EventBeginPlay
  (if (not (Variables|Default|GetIsPreview))
    (Game|SpawnActorfromClass "/Game/Blueprint/IA/BP_Minpik.BP_Minpik_C" (Math|Conversions|ToTransform(Vector) (Transformation|GetActorLocation self)) "Undefined" "MultiplyWithRoot" 0 "NewEnumerator1" 0)
    (Default|CheckGameState (.AsBP%20Game%20Mode (Utilities|Casting|CastToBP_GameMode (Game|GetGameMode))))))

(fn ConstructionScript
  (|CallParentFunction))